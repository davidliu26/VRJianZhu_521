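; BP_UILogic is an actor that drives UI flow and day/night lighting toggling.
; BeginPlay shows the WBP_Login widget with the mouse cursor, and OpenMainUMG swaps it for WBP_Main.
; The F key alternates via FlipFlop between day and night by asynchronously unloading one lighting streaming level and loading the other, BuildEntry_DayLight or BuildEntry_NightLight.
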(event Custom|OpenMainUMG
  (Widget|RemovefromParent (Variables|UMG|GetWBP_Login_UMG))
  (bind _returnvalue (UserInterface|CreateWidget "/Game/UI/UMG/WBP_Main.WBP_Main_C"))
  (bind _output_get (Variables|UMG|SetWBP_Main_UMG _returnvalue))
  (UserInterface|Viewport|AddtoViewport _output_get 0))

(event Custom|SwitchDay2Night
  (Class|GameplayStatics|UnloadStreamLevelbySoftObjectPtr "/Game/Map/BuildEntry_DayLight.BuildEntry_DayLight" false)
  (Class|GameplayStatics|LoadStreamLevelbySoftObjectPtr "/Game/Map/BuildEntry_NightLight.BuildEntry_NightLight" true false))

(event Custom|SwitchNight2Day
  (Class|GameplayStatics|UnloadStreamLevelbySoftObjectPtr "/Game/Map/BuildEntry_NightLight.BuildEntry_NightLight" false)
  (Class|GameplayStatics|LoadStreamLevelbySoftObjectPtr "/Game/Map/BuildEntry_DayLight.BuildEntry_DayLight" true false))

(event EventBeginPlay
  (bind _returnvalue (UserInterface|CreateWidget "/Game/UI/UMG/WBP_Login.WBP_Login_C"))
  (bind _output_get (Variables|UMG|SetWBP_Login_UMG _returnvalue))
  (UserInterface|Viewport|AddtoViewport _output_get 0)
  (Variables|/Script/Engine.PlayerController|SetbShowMouseCursor (Game|GetPlayerController 0) true))

(event Input|KeyboardEvents|F
  (params (Key :type Key%20Structure :default "None"))
  (:Pressed
    (Utilities|FlowControl|FlipFlop
      (:A
        (CallFunction|SwitchDay2Night))
      (:B
        (CallFunction|SwitchNight2Day)))))

(fn ConstructionScript)